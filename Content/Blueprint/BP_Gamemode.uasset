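; Game mode for local multiplayer that sets up player slots, the menu and character spawning.
; On BeginPlay it matches numeric PlayerStart tags to player indices, creates local players, possesses a Bp_InputReceiver at each start, then shows WBP_Menu.
; DisplayCharacterSelect adds a per-player selection widget and hands it to that player's receiver.
; Spawnplayer spawns BP_Player with the chosen character at the receiver's transform and transfers possession to it.
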(event EventBeginPlay
  (CallFunction|GetPlayerStartPoints)
  (CallFunction|SpawnInputReceivers)
  (bind _returnvalue (UserInterface|CreateWidget "/Game/Blueprint/UI/WBP_Menu.WBP_Menu_C"))
  (bind _output_get (Variables|Default|SetMenuWidgetRef _returnvalue))
  (UserInterface|Viewport|AddtoViewport _output_get 0))

(fn ConstructionScript)

(fn GetPlayerStartPoints
  (bind _outactors (Actor|GetAllActorsOfClass "/Script/Engine.PlayerStart"))
  (Variables|Default|SetPlayer%20Start%20Array _outactors))

(fn SpawnInputReceivers
  (for (_ _array_index) (Variables|Default|GetPlayer%20Start%20Array)
    (LocalVariables|SetIndex _array_index)
    (for _array_element (Variables|Default|GetPlayer%20Start%20Array)
      (if (== (CallFunction|NametoInt _array_element) (LocalVariables|GetIndex))
        (Class|GameplayStatics|CreatePlayer -1)
        (bind _returnvalue (Game|SpawnActorfromClass "/Game/Blueprint/Bp_InputReceiver.Bp_InputReceiver_C" (Transformation|GetActorTransform (Utilities|Array|Get(acopy) (Variables|Default|GetPlayer%20Start%20Array) (LocalVariables|GetIndex))) "Undefined" 0 (LocalVariables|GetIndex) 0))
        (Utilities|Array|AddUnique (Variables|Default|GetPlayerInputReceiverArray) _returnvalue)
        (Pawn|Possess (Game|GetPlayerController (LocalVariables|GetIndex)) _returnvalue)
        (Utilities|Array|AddUnique (Variables|Default|GetPlayerControllerArray) (Game|GetPlayerController (LocalVariables|GetIndex)))))))

(fn NametoInt
  (params (PlayerStart :type Player%20Start%20Object%20Reference))
  (return (Math|Conversions|ToInteger(Byte) (Utilities|String|ToString(Name) (Variables|/Script/Engine.PlayerStart|GetPlayerStartTag PlayerStart)))))

(fn DisplayCharacterSelect
  (params (CurrentPlayerInd :type Integer))
  (bind _characterselect (Default|AddCharacterSelect (Variables|Default|GetMenuWidgetRef) CurrentPlayerInd))
  (Variables|/Game/Blueprint/Bp_InputReceiver.Bp_InputReceiver_C|SetCharcterMenuRef (Utilities|Array|Get(acopy) (Variables|Default|GetPlayerInputReceiverArray) CurrentPlayerInd) _characterselect)
  (return false))

(fn Spawnplayer
  (params (CurrentPlayerInd :type Integer) (InputReceiver :type Bp%20Input%20Receiver%20Object%20Reference) (CharacterChoice :type Integer))
  (bind _returnvalue (Game|SpawnActorfromClass "/Game/Blueprint/BP_Player.BP_Player_C" (Transformation|GetActorTransform InputReceiver) "Undefined" 0 CharacterChoice 0))
  (Pawn|Possess (Game|GetPlayerController CurrentPlayerInd) _returnvalue)
  (return false))