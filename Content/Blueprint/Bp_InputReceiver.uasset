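; Bp_InputReceiver handles one player's join and character-select input in what appears to be a local multiplayer lobby.
; Start asks the GameMode to display the character select message for its PlayerIndex when no menu reference is valid.
; With a valid menu, Start sends the chosen character and itself to the GameMode's spawn message, then removes and clears the menu.
; Left and Right inputs cycle the menu's character in opposite directions.
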(event Input|ActionEvents|InputActionStart
  (params (Key :type Key%20Structure :default "None"))
  (:Pressed
    (Utilities|IsValid (Variables|Default|GetCharcterMenuRef)
      (:Is%20Valid
        (Class|BPIGamemode|Spawnplayer(Message) (Game|GetGameMode) (Variables|Default|GetPlayerIndex) self (Variables|/Game/Blueprint/UI/WBP_CharacterSelect.WBP_CharacterSelect_C|GetCharacterChoices (Variables|Default|GetCharcterMenuRef)))
        (Widget|RemovefromParent (Variables|Default|GetCharcterMenuRef))
        (Variables|Default|SetCharcterMenuRef 0))
      (:Is%20Not%20Valid
        (Class|BPIGamemode|DisplayCharacterSelect(Message) (Game|GetGameMode) (Variables|Default|GetPlayerIndex))))))

(event Input|ActionEvents|InputActionIA_Select_Left
  (params (Key :type Key%20Structure :default "None"))
  (:Pressed
    (Utilities|IsValid (Variables|Default|GetCharcterMenuRef)
      (:Is%20Valid
        (Default|SwichCharacter (Variables|Default|GetCharcterMenuRef) 1)))))

(event Input|ActionEvents|InputActionIA_Select_Right
  (params (Key :type Key%20Structure :default "None"))
  (:Pressed
    (Utilities|IsValid (Variables|Default|GetCharcterMenuRef)
      (:Is%20Valid
        (Default|SwichCharacter (Variables|Default|GetCharcterMenuRef) -1)))))

(fn ConstructionScript)